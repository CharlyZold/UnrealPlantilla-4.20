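; Grabbable VR bow that spawns a BP_Holder as the string grip and launches a nocked arrow when that holder is released.
; Gripping the bow enables the holder's grab; releasing either snaps the holder back to the bow.
; Each tick, holder position aims the arrow and sets the anim blueprint's pull amount, two bowstring splines and haptic strength.
; Firing detaches ArrowRef, enables physics and derives velocity from the holder-to-ArrowDirection-socket vector.
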(event Custom|Grabbed
  (bind _returnvalue (Math|Transform|MakeTransform "0, 0, 0"))
  (bind _holderref (Variables|Default|GetHolderRef))
  (bind _grabable (Variables|/Game/Blueprints/BP_Holder.BP_Holder_C|GetGrabable _holderref))
  (Default|SetFixedGrab _grabable (Variables|/Game/Blueprints/BP_Holder.BP_Holder_C|GetSphere _holderref) _returnvalue "/Game/Playground/HandPoses/hand_pose_cup.hand_pose_cup" _returnvalue)
  (EventDispatchers|BindEventtoReleaseNotify _grabable (delegate Custom|HolderReleased)))

(event Custom|Released
  (Default|ClearGrab (Variables|/Game/Blueprints/BP_Holder.BP_Holder_C|GetGrabable (Variables|Default|GetHolderRef)))
  (CallFunction|AttacharHolder))

(event Custom|HolderReleased
  (Audio|PlaySoundatLocation "/Game/Playground/Objects/Bow/bow.bow" (Transformation|GetActorLocation (Variables|Default|GetHolderRef)) "0, 0, 0" 6.0 1.0 0.0 0 0 0)
  (Utilities|IsValid (Variables|Default|GetArrowRef)
    (:Is%20Valid
      (CallFunction|FireArrg))
    (:Is%20Not%20Valid
      _))
  (CallFunction|AttacharHolder))

(event EventBeginPlay
  (bind _grabable (Variables|Default|GetGrabable))
  (Default|SetFixedGrab (Variables|Default|GetGrabable) (Variables|Default|GetBow) (Math|Transform|MakeTransform "0.000000,6.000000,7.000000" "-110.000000,110.000000,0.000000") "/Game/Modelado/Bow_Rig+Anim_Anim.Bow_Rig+Anim_Anim" (Math|Transform|MakeTransform "0, 0, 0"))
  (bind _returnvalue (Game|SpawnActorfromClass "/Game/Blueprints/BP_Holder.BP_Holder_C" (Math|Transform|MakeTransform "0, 0, 0") "Undefined" 0 0))
  (bind _output_get (Variables|Default|SetHolderRef _returnvalue))
  (bind _output_get_2 (Variables|/Game/Blueprints/BP_Holder.BP_Holder_C|SetBowRef _output_get self))
  (CallFunction|AttacharHolder _output_get_2)
  (EventDispatchers|BindEventtoGrabNotify _grabable (delegate Custom|Grabbed))
  (EventDispatchers|BindEventtoReleaseNotify _grabable (delegate Custom|Released)))

(event EventTick
  (params (DeltaSeconds :type Float%20%28single-precision%29))
  (CallFunction|ArrowUpdate)
  (CallFunction|AnimUpdate))

(fn ConstructionScript)

(fn AttacharHolder
  (bind _holderref (Variables|Default|GetHolderRef))
  (Transformation|DetachFromActor _holderref "KeepRelative" "KeepRelative" "KeepRelative")
  (Transformation|AttachActorToActor _holderref self "None" "SnapToTarget" "SnapToTarget" "SnapToTarget" true)
  (Transformation|AddActorLocalOffset _holderref "-166.000000,0.000000, 0" false false))

(fn FireArrg
  (bind _holderref (Variables|Default|GetHolderRef))
  (bind _bow (Variables|Default|GetBow))
  (bind _returnvalue (Transformation|GetActorLocation _holderref))
  (bind _returnvalue_2 (Transformation|GetSocketLocation _bow "ArrowDirection"))
  (bind _returnvalue_3 (- _returnvalue_2 _returnvalue))
  (Transformation|DetachFromActor (Variables|Default|GetArrowRef) "KeepWorld" "KeepWorld" "KeepWorld")
  (Physics|SetSimulatePhysics (Variables|/Game/Blueprints/BP_Flecha.BP_Flecha_C|GetStaticFlecha (Variables|Default|GetArrowRef)) true)
  (Physics|SetEnableGravity (Variables|/Game/Blueprints/BP_Flecha.BP_Flecha_C|GetStaticFlecha (Variables|Default|GetArrowRef)) true)
  (Physics|SetPhysicsLinearVelocity (Variables|/Game/Blueprints/BP_Flecha.BP_Flecha_C|GetStaticFlecha (Variables|Default|GetArrowRef)) (+ (* _returnvalue_3 1.2e+02) (* (Math|Vector|Normalize _returnvalue_3) -1.2e+03)) true "None")
  (Default|Setup (Variables|Default|GetArrowRef))
  (Variables|Default|SetArrowRef 0))

(fn AnimUpdate
  (bind _holderref (Variables|Default|GetHolderRef))
  (bind _string1 (Variables|Default|GetString1))
  (bind _string2 (Variables|Default|GetString2))
  (bind _bow (Variables|Default|GetBow))
  (bind _bow_2 (Variables|Default|GetBow))
  (bind _returnvalue (Transformation|GetSocketLocation _bow_2 "BowstringTop"))
  (bind _returnvalue_2 (Transformation|GetSocketLocation _bow "BowstringBot"))
  (bind _grabable (Variables|/Game/Blueprints/BP_Holder.BP_Holder_C|GetGrabable _holderref))
  (bind _asbow_anim_bp (Utilities|Casting|CastToBowAnimBP (Components|SkeletalMesh|GetAnimInstance (Variables|Default|GetBow))))
  (bind _output_get (Variables|/Game/Playground/Objects/Bow/BowAnimBP.BowAnimBP_C|SetPulled _asbow_anim_bp (Math|Float|Clamp(Float) (Math|Float|Power (/ (Math|Vector|VectorLength (- (Math|Transform|TransformLocation (Math|Transform|InvertTransform (Transformation|GetActorTransform self)) (Transformation|GetActorLocation (Variables|Default|GetHolderRef))) "0,-13.000000, 0")) 8e+01) 0.4))))
  (LocalVariables|SetPullScale _output_get)
  (SplineMesh|SetStartPosition _string1 (Math|Transform|TransformLocation (Transformation|GetActorTransform (Variables|Default|GetHolderRef)) (Math|Vector|MakeVector -2.5 0.0 0.0)) false)
  (SplineMesh|SetEndPosition _string1 _returnvalue_2 true)
  (SplineMesh|SetEndTangent _string1 (* (* (Math|Vector|Normalize (- _returnvalue_2 (Math|Transform|TransformLocation (Transformation|GetActorTransform) "0,-60.000000, 0"))) 45.0) (- 1.0 (LocalVariables|GetPullScale))) true :!class /Script/Engine.SplineMeshComponent)
  (SplineMesh|SetStartTangent _string1 (* (* (Math|Vector|GetForwardVector (Transformation|GetActorRotation (Variables|Default|GetHolderRef))) -4e+01) (- 1.0 (LocalVariables|GetPullScale))) true :!class /Script/Engine.SplineMeshComponent)
  (SplineMesh|SetStartPosition _string2 (Math|Transform|TransformLocation (Transformation|GetActorTransform (Variables|Default|GetHolderRef)) (Math|Vector|MakeVector 2.5 0.0 0.0)) false)
  (SplineMesh|SetEndPosition _string2 _returnvalue true)
  (SplineMesh|SetEndTangent _string2 (* (* (Math|Vector|Normalize (- _returnvalue (Math|Transform|TransformLocation (Transformation|GetActorTransform) "0,-60.000000, 0"))) 45.0) (- 1.0 (LocalVariables|GetPullScale))) true :!class /Script/Engine.SplineMeshComponent)
  (SplineMesh|SetStartTangent _string2 (* (* (Math|Vector|GetForwardVector (Transformation|GetActorRotation (Variables|Default|GetHolderRef))) 4e+01) (- 1.0 (LocalVariables|GetPullScale))) true :!class /Script/Engine.SplineMeshComponent)
  (if (Default|IsGrabbed _grabable)
    (Class|PlayerController|PlayHapticEffect (Game|GetPlayerController 0) "/Game/Playground/Objects/Bow/BowTreble.BowTreble" (Variables|/Game/Framework/Hands/HandBP.HandBP_C|GetHandType (Variables|/Game/Framework/Hands/Grabable.Grabable_C|GetHand _grabable)) (* (Math|Float|Clamp(Float) (- (LocalVariables|GetPullScale) 0.5)) 2.0) false)))

(fn ArrowUpdate
  (bind _holderref (Variables|Default|GetHolderRef))
  (bind _arrowref (Variables|Default|GetArrowRef))
  (bind _returnvalue (Transformation|GetActorLocation _holderref))
  (Utilities|IsValid _arrowref
    (:Is%20Valid
      (Transformation|SetActorLocation _arrowref _returnvalue false false)
      (Transformation|SetActorRotation _arrowref (Math|Rotator|MakeRotfromY (Math|Vector|NegateVector (- (Transformation|GetSocketLocation (Variables|Default|GetBow) "ArrowDirection") _returnvalue)))))))