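; BP_Flecha is a hand-grabbable arrow that nocks onto a bow and sticks into what it hits.
; Touching a grabbed bow's BP_Holder while held attaches the arrow and transfers the hand's grab to the holder.
; In fast simulated flight it aligns to velocity and shows particles, with audio volume scaled by speed.
; Fast hits on non-simulating actors, except bows, holders and arrows, attach and freeze it at speed-based depth.
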(event OnComponentBeginOverlap(Sphere)
  (params (OverlappedComponent :type Primitive%20Component%20Object%20Reference) (OtherActor :type Actor%20Object%20Reference) (OtherComp :type Primitive%20Component%20Object%20Reference) (OtherBodyIndex :type Integer) (bFromSweep :type Boolean) (SweepResult :type Hit%20Result%20Structure%20%28by%20ref%29))
  (bind _asbp_holder (Utilities|Casting|CastToBP_Holder OtherActor))
  (if (and (Default|IsGrabbed (Variables|/Game/Blueprints/Bp_Bow.Bp_Bow_C|GetGrabable (Variables|/Game/Blueprints/BP_Holder.BP_Holder_C|GetBowRef _asbp_holder))) (Default|IsGrabbed (Variables|Default|GetGrabable)))
    (CallFunction|BowAttach _asbp_holder)))

(event Custom|Grabbed
  (bind _grabable (Variables|Default|GetGrabable))
  (Variables|/Game/Framework/Hands/Grabable.Grabable_C|SetSimulationPhysics _grabable true)
  (Variables|/Game/Framework/Hands/Grabable.Grabable_C|SetGravityEnabled _grabable true))

(event EventBeginPlay
  (CallFunction|Setup)
  (EventDispatchers|BindEventtoGrabNotify (Variables|Default|GetGrabable) (delegate Custom|Grabbed)))

(event Collision|EventActorBeginOverlap
  (params (OtherActor :type Actor%20Object%20Reference)))

(event EventTick
  (params (DeltaSeconds :type Float%20%28single-precision%29))
  (bind _staticflecha (Variables|Default|GetStaticFlecha))
  (bind _particlesystem (Variables|Default|GetParticleSystem))
  (bind _returnvalue (Class|PrimitiveComponent|GetPhysicsLinearVelocityatPoint _staticflecha (Transformation|GetActorLocation) "None"))
  (Variables|Default|SetVelocidad _returnvalue)
  (Audio|Components|Audio|SetVolumeMultiplier (Variables|Default|GetAudio) (Math|Float|Clamp(Float) (/ (- (Math|Vector|VectorLength _returnvalue) 1e+03) 1.5e+04) 0.0 3.0) :!class /Script/Engine.AudioComponent)
  (if (and (> (Math|Vector|VectorLength _returnvalue) 2e+03) (Physics|IsSimulatingPhysics _staticflecha "None"))
    (Components|Activation|Activate _particlesystem false)
    (Transformation|SetActorRotation (Math|Rotator|MakeRotfromY _returnvalue))
    (else
      (Components|Activation|Deactivate _particlesystem))))

(event Collision|EventHit
  (params (MyComp :type Primitive%20Component%20Object%20Reference) (Other :type Actor%20Object%20Reference) (OtherComp :type Primitive%20Component%20Object%20Reference) (bSelfMoved :type Boolean) (HitLocation :type Vector :default "0, 0, 0") (HitNormal :type Vector :default "0, 0, 0") (NormalImpulse :type Vector :default "0, 0, 0") (Hit :type Hit%20Result%20Structure%20%28by%20ref%29))
  (bind _staticflecha (Variables|Default|GetStaticFlecha))
  (bind _velocidad (Variables|Default|GetVelocidad))
  (bind _returnvalue (Math|Vector|VectorLength _velocidad))
  (if (> _returnvalue 8e+02)
    (Utilities|IsValid Other
      (:Is%20Valid
        (Utilities|Casting|CastToBp_Bow Other
          (:CastFailed
            (Utilities|Casting|CastToBP_Holder Other
              (:CastFailed
                (Utilities|Casting|CastToBP_Flecha Other
                  (:CastFailed
                    (if (not (Physics|IsSimulatingPhysics (Variables|/Script/Engine.Actor|GetRootComponent Other) "None"))
                      (Transformation|AttachActorToActor Other "None" "SnapToTarget" "SnapToTarget" "KeepWorld" true)
                      (Transformation|SetActorRotation (Math|Rotator|MakeRotfromY _velocidad) :!label _label)
                      (Transformation|SetActorLocation (+ (* (Math|Vector|Normalize _velocidad) (+ (/ _returnvalue 2e+02) -7e+01)) HitLocation) false false)
                      (Physics|SetSimulatePhysics _staticflecha false)
                      (Physics|SetEnableGravity _staticflecha false)))))))))
      (:Is%20Not%20Valid
        (goto _label)))))

(fn ConstructionScript)

(fn Setup
  (Default|SetFixedGrab (Variables|Default|GetGrabable) (Variables|Default|GetStaticFlecha) (Math|Transform|MakeTransform "0.910000,1.180000,7.440000" "3.500000,60.000000,-83.000000") "/Game/Playground/HandPoses/hand_pose_cup.hand_pose_cup" (Math|Transform|MakeTransform "0.750000,0.410000,6.770000" "0.795000,-66.080002,79.650002")))

(fn BowAttach
  (params (Holder :type BP%20Holder%20Object%20Reference))
  (bind _grabable (Variables|Default|GetGrabable))
  (LocalVariables|SetHand (Variables|/Game/Framework/Hands/Grabable.Grabable_C|GetHand _grabable))
  (Default|ClearGrab _grabable)
  (Transformation|AttachActorToActor Holder "None" "SnapToTarget" "KeepWorld" "KeepWorld" true)
  (Variables|/Game/Blueprints/Bp_Bow.Bp_Bow_C|SetArrowRef (Variables|/Game/Blueprints/BP_Holder.BP_Holder_C|GetBowRef Holder) self)
  (Default|GrabObject (LocalVariables|GetHand) Holder))